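; Game mode for the Gatcha local multiplayer game that spawns and wires up the number of players set in the game instance.
; The first eight players share gamepad InputControllers in pairs, split by button set, while extra players use keyboard bindings on controller 0.
; Pawns are placed at "Player"+index PlayerStarts, then camera managers and CameraActors are destroyed.
; Tick movement and timed speed-up call empty functions, their logic left disconnected.
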(event `self.ReceiveBeginPlay`
  (`self.SpawnPlayers`)
  (`KismetSystemLibrary.K2_SetTimer` self "IncreaseSpeed" 1.0 true))

(event `self.ReceiveTick`
  (params (DeltaSeconds :type "Float (single-precision)"))
  (`self.MoveAllPlayers` DeltaSeconds))

(fn ` GetRightSpawnTransform`
  (params (Controller :type "Controller Object Reference") (Index :type Integer))
  (returns (Transform :type "Transform Structure"))
  (return (`self.GetTransform` (`self.K2_FindPlayerStart` Controller (`KismetStringLibrary.Concat_StrStr` "Player" (`KismetStringLibrary.Conv_IntToString` Index))))))

(fn `AsignAuxiPlayerToController`
  (params (PlayerIndex :type Integer) (Player :type "/Game/GatchaAsset/Prog/player Object Reference") (Controller :type "/Game/GatchaAsset/Prog/InputController Object Reference"))
  (bind _inputs (`self.GetAuxiInputStructByIndex` PlayerIndex))
  (if (not (`self.Even` PlayerIndex))
    (set `/Game/GatchaAsset/Prog/InputController.AuxiPlayer1` Player Controller)
    (set `/Game/GatchaAsset/Prog/InputController.AuxiInputPlayer1` _inputs Controller)
    (else
      (set `/Game/GatchaAsset/Prog/InputController.AuxiPlayer2` Player Controller)
      (set `/Game/GatchaAsset/Prog/InputController.AuxiInputPlayer2` _inputs Controller))))

(fn `AsignPlayersToController`
  (params (PlayerIndex :type Integer) (Player :type "/Game/GatchaAsset/Prog/player Object Reference") (Controller :type "/Game/GatchaAsset/Prog/InputController Object Reference"))
  (bind _inputs (`self.GetInputStructByIndex_Gamepad` PlayerIndex))
  (if (`self.Even` PlayerIndex)
    (set `/Game/GatchaAsset/Prog/InputController.Player1` Player Controller)
    (set `/Game/GatchaAsset/Prog/InputController.InputPlayer1` _inputs Controller)
    (else
      (set `/Game/GatchaAsset/Prog/InputController.Player2` Player Controller)
      (set `/Game/GatchaAsset/Prog/InputController.InputPlayer1` _inputs Controller))))

(fn `Even`
  (params (Value :type Integer))
  (returns (Even :type Boolean))
  (return (== (mod Value 2) 0)))

(fn `GetAuxiInputStructByIndex`
  (params (Index :type Integer))
  (returns (Inputs :type "/Game/GatchaAsset/Prog/PlayerInputStruct Structure"))
  (if (`self.Even` Index)
    (return (make `/Game/GatchaAsset/Prog/PlayerInputStruct` "Z" "S" "D" "Q"))
    (else
      (return (make `/Game/GatchaAsset/Prog/PlayerInputStruct` "Up" "Down" "Right" "Left")))))

(fn `GetControllerIndex`
  (params (PlayerIndex :type Integer))
  (returns (ControllerIndex :type Integer))
  (return (`KismetMathLibrary.FFloor` (/ (`KismetMathLibrary.Conv_IntToDouble` PlayerIndex) 2.0))))

(fn `GetInputStructByIndex_Gamepad`
  (params (index :type Integer))
  (returns (Inputs :type "/Game/GatchaAsset/Prog/PlayerInputStruct Structure"))
  ;[1 1 1] Left/Right Gamepad
  (if (`self.Even` index)
    (return (make `/Game/GatchaAsset/Prog/PlayerInputStruct` "Gamepad_DPad_Up"))
    (else
      (return (make `/Game/GatchaAsset/Prog/PlayerInputStruct` "Gamepad_FaceButton_Top" "Gamepad_FaceButton_Bottom" "Gamepad_FaceButton_Right" "Gamepad_FaceButton_Left")))))

(fn `IncreaseSpeed`)

(fn `MoveAllPlayers`
  (params (DeltaTime :type "Float (double-precision)")))

(fn `RemoveUselessActor`
  (bind _outactors (`GameplayStatics.GetAllActorsOfClass` "/Script/Engine.PlayerCameraManager"))
  (for _array_element _outactors
    (`self.K2_DestroyActor` _array_element))
  (bind _outactors_2 (`GameplayStatics.GetAllActorsOfClass` "/Script/Engine.CameraActor"))
  (for _array_element_2 _outactors_2
    (`self.K2_DestroyActor` _array_element_2)))

(fn `SafeResetPlayerPosition`
  (params (PlayerNumber :type Integer))
  (for _index (range (+ PlayerNumber 1))
    (bind _returnvalue (`GameplayStatics.GetPlayerPawn` _index))
    (`/Engine/EditorBlueprintResources/StandardMacros.IsValid` _returnvalue
      (:`Is Valid`
        (`self.K2_SetActorTransform` _returnvalue (`self. GetRightSpawnTransform` null _index) false false)))))

(fn `SetupController`
  (params (ControllerIndex :type Integer))
  (returns (Controller :type "/Game/GatchaAsset/Prog/InputController Object Reference"))
  (bind _returnvalue (`GameplayStatics.GetPlayerController` ControllerIndex))
  (`/Engine/EditorBlueprintResources/StandardMacros.IsValid` _returnvalue
    (:`Is Valid`
      (bind _asinput_controller (cast `/Game/GatchaAsset/Prog/InputController` _returnvalue))
      (return _asinput_controller))
    (:`Is Not Valid`
      (bind _returnvalue_2 (`GameplayStatics.CreatePlayer` ControllerIndex))
      (bind _asinput_controller_2 (cast `/Game/GatchaAsset/Prog/InputController` _returnvalue_2))
      (set `/Game/GatchaAsset/Prog/InputController.Index` ControllerIndex _asinput_controller_2)
      (return _asinput_controller_2))))

(fn `SetupControllerAndPlayer_Gamepad`
  (params (IndexPlayer :type Integer) (IndexController :type Integer) (NbMaxPlayer :type Integer))
  (locals (TempIndexPlayer :type Integer) (TempInputController :type "/Game/GatchaAsset/Prog/InputController Object Reference") (TempIndexController :type Integer) (TempMaxPlayer :type Integer))
  (set `local.TempIndexPlayer` IndexPlayer)
  (set `local.TempIndexController` IndexController)
  (set `local.TempMaxPlayer` NbMaxPlayer)
  (bind _controller (`self.SetupController` (`local.TempIndexController`)))
  (bind (_index _player _attachedcontroller) (`self.SetupPlayer` (`local.TempIndexPlayer`) _controller))
  (`self.AsignPlayersToController` _index _player _attachedcontroller)
  (`self.SafeResetPlayerPosition` (`local.TempMaxPlayer`)))

(fn `SetupPlayer`
  (params (PlayerIndex :type Integer) (Controller :type "/Game/GatchaAsset/Prog/InputController Object Reference"))
  (returns (Index :type Integer) (Player :type "/Game/GatchaAsset/Prog/player Object Reference") (AttachedController :type "/Game/GatchaAsset/Prog/InputController Object Reference"))
  (bind _returnvalue (`GameplayStatics.GetPlayerPawn` PlayerIndex))
  (`/Engine/EditorBlueprintResources/StandardMacros.IsValid` _returnvalue
    (:`Is Valid`
      (bind _asplayer (cast `/Game/GatchaAsset/Prog/player` _returnvalue))
      (return PlayerIndex _asplayer Controller))
    (:`Is Not Valid`
      (bind _returnvalue_2 (`|SpawnActorFromClass` "/Game/GatchaAsset/Prog/player.Player_C" (`self. GetRightSpawnTransform` null PlayerIndex) "AlwaysSpawn" "OverrideRootScale" null null))
      (return PlayerIndex _returnvalue_2 Controller))))

(fn `SpawnPlayers`
  ;[1 1 1] SpawnPlayers
  (bind _asgatcha_game_instance (cast `/Game/GatchaAsset/Prog/GatchaGameInstance` (`GameplayStatics.GetGameInstance`)))
  (for _index (range (`/Game/GatchaAsset/Prog/GatchaGameInstance.NbPlayers` _asgatcha_game_instance))
    (if (< _index 8)
      ;;[1 0 0] For Gamepad
      (`self.SetupControllerAndPlayer_Gamepad` _index (`self.GetControllerIndex` _index) (`/Game/GatchaAsset/Prog/GatchaGameInstance.NbPlayers` _asgatcha_game_instance))
      (else
        ;;[0 0 1] For keypad
        (bind _asinput_controller (cast `/Game/GatchaAsset/Prog/InputController` (`GameplayStatics.GetPlayerController` 0)))
        (bind (_index_2 _player _attachedcontroller) (`self.SetupPlayer` _index _asinput_controller))
        (`self.AsignAuxiPlayerToController` _index_2 _player _attachedcontroller))))
  (`self.RemoveUselessActor`))

(fn `UserConstructionScript`)