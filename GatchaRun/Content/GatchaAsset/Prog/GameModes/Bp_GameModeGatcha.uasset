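; Game mode for a local multiplayer auto-scrolling game, running the round from main menu to end menu.
; AddPlayer spawns players at indexed PlayerStarts, pairing two per InputController; SpawnPlayers also maps split-gamepad and keyboard bindings.
; Tick pushes players and camera forward at LevelSpeed, which a looping timer compounds once StartLevel runs.
; It relays score and HP to GameUI, records scores on death and ends the round when one player remains.
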(event `self.ReceiveBeginPlay`
  (bind _returnvalue (`GameplayStatics.GetPlayerController` 0))
  (`|ExecutionSequence`
    (:`then_0`
      (bind _returnvalue_2 (`|CreateWidget` "/Game/GatchaAsset/Ui/MainMenu.MainMenu_C" _returnvalue))
      (`UserWidget.AddToViewport` _returnvalue_2 0)
      (`WidgetBlueprintLibrary.SetInputMode_GameAndUIEx` _returnvalue _returnvalue_2 "DoNotLock" false)
      (set `PlayerController.bShowMouseCursor` true _returnvalue)
      (set `self.LevelSpeed` 0.0)
      (`self.AddPlayer`))
    (:`then_1`
      (bind _returnvalue_3 (`|CreateWidget` "/Game/GatchaAsset/Ui/EndMenu.EndMenu_C"))
      (set `self.EndMenu` _returnvalue_3))))

(event `self.ReceiveTick`
  (params (DeltaSeconds :type "Float (single-precision)"))
  (`self.MoveAllPlayers` DeltaSeconds))

(fn ` GetRightSpawnTransform`
  (params (Controller :type "Controller Object Reference") (Index :type Integer))
  (returns (Transform :type "Transform Structure"))
  (return (`self.GetTransform` (`self.K2_FindPlayerStart` Controller (`KismetStringLibrary.Concat_StrStr` "Player" (`KismetStringLibrary.Conv_IntToString` Index))))))

(fn `addHpPlayer`
  (params (playerIndex :type Integer))
  (bind _foundwidgets (`WidgetBlueprintLibrary.GetAllWidgetsOfClass` "/Game/GatchaAsset/Ui/GameUI.GameUI_C"))
  (`/Game/GatchaAsset/Ui/GameUI.addHP` (`|GetArrayItem` _foundwidgets) playerIndex))

(fn `AddPlayer`
  (bind _nbplayers (`self.nbPlayers`))
  (bind _controller (`self.SetupController` (`self.GetControllerIndex` _nbplayers)))
  (bind (_index _player) (`self.SetupPlayer` _nbplayers))
  (`/Game/GatchaAsset/Prog/Character/InputController.AddPlayer` _controller _player)
  (`/Engine/EditorBlueprintResources/StandardMacros.IncrementInt` (`self.nbPlayers`)))

(fn `AsignAuxiPlayerToController`
  (params (PlayerIndex :type Integer) (Player :type "/Game/GatchaAsset/Prog/Character/MyPlayer Object Reference") (Controller :type "/Game/GatchaAsset/Prog/Character/InputController Object Reference"))
  (bind _inputs (`self.GetAuxiInputStructByIndex` PlayerIndex))
  (if (not (`self.Even` PlayerIndex))
    (set `/Game/GatchaAsset/Prog/Character/InputController.AuxiPlayer1` Player Controller)
    (set `/Game/GatchaAsset/Prog/Character/InputController.AuxiInputPlayer1` _inputs Controller)
    (else
      (set `/Game/GatchaAsset/Prog/Character/InputController.AuxiPlayer2` Player Controller)
      (set `/Game/GatchaAsset/Prog/Character/InputController.AuxiInputPlayer2` _inputs Controller))))

(fn `AsignPlayersToController`
  (params (PlayerIndex :type Integer) (Player :type "/Game/GatchaAsset/Prog/Character/MyPlayer Object Reference") (Controller :type "/Game/GatchaAsset/Prog/Character/InputController Object Reference"))
  (bind _inputs (`self.GetInputStructByIndex_Gamepad` PlayerIndex))
  (if (`self.Even` PlayerIndex)
    (set `/Game/GatchaAsset/Prog/Character/InputController.Player1` Player Controller)
    (set `/Game/GatchaAsset/Prog/Character/InputController.InputPlayer1` _inputs Controller)
    (else
      (set `/Game/GatchaAsset/Prog/Character/InputController.Player2` Player Controller)
      (set `/Game/GatchaAsset/Prog/Character/InputController.InputPlayer1` _inputs Controller))))

(fn `EndRound`
  (bind _returnvalue (`GameplayStatics.GetPlayerController` 0))
  (bind _endmenu (`self.EndMenu`))
  (`WidgetLayoutLibrary.RemoveAllWidgets`)
  (`UserWidget.AddToViewport` _endmenu 0)
  (`WidgetBlueprintLibrary.SetInputMode_UIOnlyEx` _returnvalue _endmenu)
  (set `PlayerController.bShowMouseCursor` true _returnvalue)
  (`/Game/GatchaAsset/Ui/EndMenu.update` _endmenu (`self.scores`) (`self.indexes`)))

(fn `Even`
  (params (Value :type Integer))
  (returns (Even :type Boolean))
  (return (== (mod Value 2) 0)))

(fn `GetAuxiInputStructByIndex`
  (params (Index :type Integer))
  (returns (Inputs :type "/Game/GatchaAsset/Prog/Structures/PlayerInputStruct Structure"))
  (if (`self.Even` Index)
    (return (make `/Game/GatchaAsset/Prog/Structures/PlayerInputStruct` "Z" "S" "D" "Q"))
    (else
      (return (make `/Game/GatchaAsset/Prog/Structures/PlayerInputStruct` "Up" "Down" "Right" "Left")))))

(fn `GetControllerIndex`
  (params (PlayerIndex :type Integer))
  (returns (ControllerIndex :type Integer))
  (if (>= PlayerIndex 8)
    (return 0)
    (else
      (return (`KismetMathLibrary.FFloor` (/ (`KismetMathLibrary.Conv_IntToDouble` PlayerIndex) 2.0))))))

(fn `GetInputStructByIndex_Gamepad`
  (params (index :type Integer))
  (returns (Inputs :type "/Game/GatchaAsset/Prog/Structures/PlayerInputStruct Structure"))
  ;[1 1 1] Left/Right Gamepad
  (if (`self.Even` index)
    (return (make `/Game/GatchaAsset/Prog/Structures/PlayerInputStruct` "Gamepad_DPad_Up"))
    (else
      (return (make `/Game/GatchaAsset/Prog/Structures/PlayerInputStruct` "Gamepad_FaceButton_Top" "Gamepad_FaceButton_Bottom" "Gamepad_FaceButton_Right" "Gamepad_FaceButton_Left")))))

(fn `GetScoreWinner`
  (params (Scores :type "Array of Integer") (Indexes :type "Array of Integer"))
  (returns (Score :type Integer) (PlayerIndex :type Integer))
  (locals (`Highest score` :type Integer) (Index :type Integer))
  (for (_array_element _array_index) Scores
    (if (<= (`local.Highest score`) _array_element)
      (set `local.Highest score` _array_element)
      (set `local.Index` _array_index)))
  (return (`local.Highest score`) (`|GetArrayItem` (`self.indexes`) (`local.Index`))))

(fn `IncreaseSpeed`
  (bind _output_get (set `self.LevelSpeed` (+ (/ (* (`self.IncrementValue`) (`self.LevelSpeed`)) 100.0) (`self.LevelSpeed`))))
  (`KismetSystemLibrary.PrintString` (`KismetStringLibrary.Conv_DoubleToString` _output_get) true true (struct :`G` 0.66 :`B` 1.0 :`A` 1.0) 1.0))

(fn `killPlayer`
  (params (playerIndex :type Integer))
  (bind _output (`|GetArrayItem` (`self.Players`) playerIndex))
  (`/Engine/EditorBlueprintResources/StandardMacros.IsValid` _output
    (:`Is Valid`
      (`KismetArrayLibrary.Array_Add` (`self.scores`) (`/Game/GatchaAsset/Prog/Character/MyPlayer.score` _output))
      (`KismetArrayLibrary.Array_Add` (`self.indexes`) playerIndex)
      (`self.K2_DestroyActor` (`|GetArrayItem` (`self.Players`) playerIndex))
      (if (== (`self.nbPlayers`) (+ (`self.deleted`) 2))
        (`self.EndRound`)
        (else
          (`/Engine/EditorBlueprintResources/StandardMacros.IncrementInt` (`self.deleted`)))))
    (:`Is Not Valid`
      (`KismetSystemLibrary.PrintString` "NULL INDEX :")
      (`KismetSystemLibrary.PrintString` (`KismetStringLibrary.Conv_IntToString` playerIndex)))))

(fn `MoveAllPlayers`
  (params (DeltaTime :type "Float (double-precision)"))
  (bind _levelspeed (`self.LevelSpeed`))
  (bind _cameraactor (`self.CameraActor`))
  (for _array_element (`self.Players`)
    (`/Engine/EditorBlueprintResources/StandardMacros.IsValid` _array_element
      (:`Is Valid`
        (`self.K2_SetActorLocation` _array_element (+ (* (`self.GetActorForwardVector` _array_element) (* DeltaTime _levelspeed)) (`self.K2_GetActorLocation` _array_element)) false false))))
  (`/Engine/EditorBlueprintResources/StandardMacros.IsValid` _array_element
    (:`Is Valid`
      (`self.K2_SetActorLocation` _cameraactor (+ (* (`self.GetActorForwardVector` _cameraactor) (* DeltaTime _levelspeed)) (`self.K2_GetActorLocation` _cameraactor)) false false))))

(fn `removeHpPlayer`
  (params (PlayerIndex :type Integer))
  (bind _foundwidgets (`WidgetBlueprintLibrary.GetAllWidgetsOfClass` "/Game/GatchaAsset/Ui/GameUI.GameUI_C"))
  (if (!= (`KismetArrayLibrary.Array_Length` _foundwidgets) 0)
    (`/Game/GatchaAsset/Ui/GameUI.RemoveHP` (`|GetArrayItem` _foundwidgets) PlayerIndex)))

(fn `RemovePlayer`
  (bind _output (`|GetArrayItem` (`self.Players`) (- (`self.nbPlayers`) 1)))
  (`/Game/GatchaAsset/Prog/Character/InputController.RemovePlayer` (`/Game/GatchaAsset/Prog/Character/MyPlayer.PlayerController` _output))
  (`self.K2_DestroyActor` _output)
  (`KismetArrayLibrary.Array_Remove` (`self.Players`) (- (`self.nbPlayers`) 1))
  (`/Engine/EditorBlueprintResources/StandardMacros.DecrementInt` (`self.nbPlayers`)))

(fn `RemoveUselessActor`
  (bind _outactors (`GameplayStatics.GetAllActorsOfClass` "/Script/Engine.PlayerCameraManager"))
  (for _array_element _outactors
    (`self.K2_DestroyActor` _array_element))
  (bind _outactors_2 (`GameplayStatics.GetAllActorsOfClass` "/Script/Engine.CameraActor"))
  (for _array_element_2 _outactors_2
    (`self.K2_DestroyActor` _array_element_2)))

(fn `resetScores`
  (bind _foundwidgets (`WidgetBlueprintLibrary.GetAllWidgetsOfClass` "/Game/GatchaAsset/Ui/GameUI.GameUI_C"))
  (for (_ _array_index) (`self.Players`)
    (`/Game/GatchaAsset/Ui/GameUI.updateScore` (`|GetArrayItem` _foundwidgets) 0 _array_index)))

(fn `restartLevel`
  (locals (tmp :type Integer))
  (bind _output_get (set `local.tmp` (`self.nbPlayers`)))
  (set `self.nbPlayers` 0)
  (for _ (range _output_get)
    (`self.AddPlayer`)
    (`self.StartLevel`)
    (`self.trick`)))

(fn `SafeResetPlayerPosition`
  (params (PlayerNumber :type Integer))
  (for _index (range (+ PlayerNumber 1))
    (bind _returnvalue (`GameplayStatics.GetPlayerPawn` _index))
    (`/Engine/EditorBlueprintResources/StandardMacros.IsValid` _returnvalue
      (:`Is Valid`
        (`self.K2_SetActorTransform` _returnvalue (`self. GetRightSpawnTransform` null _index) false false)))))

(fn `SetupController`
  (params (ControllerIndex :type Integer))
  (returns (Controller :type "/Game/GatchaAsset/Prog/Character/InputController Object Reference"))
  (bind _returnvalue (`GameplayStatics.GetPlayerController` ControllerIndex))
  (`/Engine/EditorBlueprintResources/StandardMacros.IsValid` _returnvalue
    (:`Is Valid`
      (bind _asinput_controller (cast `/Game/GatchaAsset/Prog/Character/InputController` _returnvalue))
      (return _asinput_controller))
    (:`Is Not Valid`
      (bind _returnvalue_2 (`GameplayStatics.CreatePlayer` ControllerIndex))
      (bind _asinput_controller_2 (cast `/Game/GatchaAsset/Prog/Character/InputController` _returnvalue_2))
      (set `/Game/GatchaAsset/Prog/Character/InputController.Index` ControllerIndex _asinput_controller_2)
      (return _asinput_controller_2))))

(fn `SetupControllerAndPlayer_Gamepad`
  (params (IndexPlayer :type Integer) (IndexController :type Integer) (NbMaxPlayer :type Integer))
  (locals (TempIndexPlayer :type Integer) (TempInputController :type "/Game/GatchaAsset/Prog/Character/InputController Object Reference") (TempIndexController :type Integer) (TempMaxPlayer :type Integer))
  (set `local.TempIndexPlayer` IndexPlayer)
  (set `local.TempIndexController` IndexController)
  (set `local.TempMaxPlayer` NbMaxPlayer)
  (bind _controller (`self.SetupController` (`local.TempIndexController`)))
  (bind (_index _player) (`self.SetupPlayer` (`local.TempIndexPlayer`)))
  (`self.AsignPlayersToController` _index _player _controller)
  (`self.SafeResetPlayerPosition` (`local.TempMaxPlayer`)))

(fn `SetupPlayer`
  (params (PlayerIndex :type Integer))
  (returns (Index :type Integer) (Player :type "/Game/GatchaAsset/Prog/Character/MyPlayer Object Reference"))
  (bind _returnvalue (`|SpawnActorFromClass` "/Game/GatchaAsset/Prog/Character/MyPlayer.MyPlayer_C" (`self. GetRightSpawnTransform` null PlayerIndex) "AlwaysSpawn" "OverrideRootScale" null null))
  (`/Game/GatchaAsset/Prog/Character/MyPlayer.SetIndexPlayer` _returnvalue PlayerIndex)
  (bind _returnvalue_2 (`KismetArrayLibrary.Array_Add` (`self.Players`) _returnvalue))
  (`KismetSystemLibrary.PrintString` (`KismetStringLibrary.Conv_IntToString` _returnvalue_2))
  (return PlayerIndex _returnvalue))

(fn `SpawnPlayers`
  ;[1 1 1] SpawnPlayers
  (cast `/Game/GatchaAsset/Prog/GameInsances/GatchaGameInstance` (`GameplayStatics.GetGameInstance`))
  (for _index (range (`self.nbPlayers`))
    (if (< _index 8)
      ;;[1 0 0] For Gamepad
      (`self.SetupControllerAndPlayer_Gamepad` _index (`self.GetControllerIndex` _index) (`self.nbPlayers`))
      (else
        ;;[0 0 1] For keypad
        (bind _asinput_controller (cast `/Game/GatchaAsset/Prog/Character/InputController` (`GameplayStatics.GetPlayerController` 0)))
        (bind (_index_2 _player) (`self.SetupPlayer` _index))
        (`self.AsignAuxiPlayerToController` _index_2 _player _asinput_controller))))
  (`self.RemoveUselessActor`))

(fn `StartLevel`
  (bind _returnvalue (`GameplayStatics.GetPlayerController` 0))
  (set `self.blockInput?` false)
  (bind _returnvalue_2 (`|CreateWidget` "/Game/GatchaAsset/Ui/GameUI.GameUI_C"))
  (`UserWidget.AddToViewport` _returnvalue_2 0)
  (`WidgetBlueprintLibrary.SetInputMode_GameOnly` _returnvalue)
  (set `PlayerController.bShowMouseCursor` false _returnvalue)
  (set `self.LevelSpeed` 250.0)
  (`KismetSystemLibrary.K2_SetTimer` self "IncreaseSpeed" 1.0 true)
  (`self.resetScores`))

(fn `UpdatePlayerScore`
  (params (playerIndex :type Integer) (Score :type Integer))
  (bind _foundwidgets (`WidgetBlueprintLibrary.GetAllWidgetsOfClass` "/Game/GatchaAsset/Ui/GameUI.GameUI_C"))
  (`/Game/GatchaAsset/Ui/GameUI.updateScore` (`|GetArrayItem` _foundwidgets) Score playerIndex))

(fn `UserConstructionScript`)