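; Game mode for a local multiplayer forward-runner with walls, managing menus, players, scores and the round lifecycle.
; Players spawn at indexed PlayerStarts, with up to ten sharing four input controllers.
; Tick moves players and camera forward at LevelSpeed, which a one-second timer raises logarithmically once StartLevel spawns the wall spawner.
; Deaths save scores and update audio until the last opens the end menu; RestartLevel respawns players and clears walls.
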(event `self.ReceiveBeginPlay`
  (`|ExecutionSequence`
    (:`then_0`
      (`self.CreateMainMenu`))
    (:`then_1`
      (`self.InstanciateControllers`))
    (:`then_2`
      (`self.AddPlayer`))
    (:`then_3`
      (set `self.LevelSpeed` 0.0))
    (:`then_4`
      (bind _returnvalue (`|CreateWidget` "/Game/GatchaAsset/Ui/EndMenu.EndMenu_C"))
      (set `self.EndMenu` _returnvalue))))

(event `self.ReceiveTick`
  (params (DeltaSeconds :type "Float (single-precision)"))
  (`self.MoveAllPlayers` DeltaSeconds))

(fn ` GetRightSpawnTransform`
  (params (Controller :type "Controller Object Reference") (Index :type Integer))
  (returns (Transform :type "Transform Structure"))
  (return (`self.GetTransform` (`self.K2_FindPlayerStart` Controller (`KismetStringLibrary.Concat_StrStr` "Player" (`KismetStringLibrary.Conv_IntToString` Index))))))

(fn `addHpPlayer`
  (params (playerIndex :type Integer))
  (bind _foundwidgets (`WidgetBlueprintLibrary.GetAllWidgetsOfClass` "/Game/GatchaAsset/Ui/GameUI.GameUI_C"))
  (`/Game/GatchaAsset/Ui/GameUI.addHP` (`|GetArrayItem` _foundwidgets) playerIndex))

(fn `AddPlayer`
  (bind _nbplayers (`self.nbPlayers`))
  (bind (_index _player) (`self.SetupPlayer` _nbplayers))
  (bind _asinput_controller (cast `/Game/GatchaAsset/Prog/Character/InputController` (`GameplayStatics.GetPlayerController` (`self.GetControllerIndex` _nbplayers))))
  (`/Game/GatchaAsset/Prog/Character/InputController.AddPlayer` _asinput_controller _player)
  (`/Engine/EditorBlueprintResources/StandardMacros.IncrementInt` (`self.nbPlayers`)))

(fn `AsignAuxiPlayerToController`
  (params (PlayerIndex :type Integer) (Player :type "/Game/GatchaAsset/Prog/Character/MyPlayer Object Reference") (Controller :type "/Game/GatchaAsset/Prog/Character/InputController Object Reference"))
  (bind _inputs (`self.GetAuxiInputStructByIndex` PlayerIndex))
  (if (not (`self.Even` PlayerIndex))
    (set `/Game/GatchaAsset/Prog/Character/InputController.AuxiPlayer1` Player Controller)
    (set `/Game/GatchaAsset/Prog/Character/InputController.AuxiInputPlayer1` _inputs Controller)
    (else
      (set `/Game/GatchaAsset/Prog/Character/InputController.AuxiPlayer2` Player Controller)
      (set `/Game/GatchaAsset/Prog/Character/InputController.AuxiInputPlayer2` _inputs Controller))))

(fn `CleanWalls`
  (`|ExecutionSequence`
    (:`then_0`
      (bind _outactors (`GameplayStatics.GetAllActorsOfClass` "/Game/GatchaAsset/Prog/Walls/BP_WallSpawner.BP_WallSpawner_C"))
      (`self.K2_DestroyActor` (`|GetArrayItem` _outactors)))
    (:`then_1`
      (bind _outactors_2 (`GameplayStatics.GetAllActorsOfClass` "/Game/GatchaAsset/Prog/Walls/BP_Wall.BP_Wall_C"))
      (for _array_element _outactors_2
        (`self.K2_DestroyActor` _array_element)))))

(fn `CreateMainMenu`
  (bind _returnvalue (`GameplayStatics.GetPlayerController` 0))
  (`WidgetLayoutLibrary.RemoveAllWidgets`)
  (bind _returnvalue_2 (`|CreateWidget` "/Game/GatchaAsset/Ui/MainMenu.MainMenu_C" _returnvalue))
  (`UserWidget.AddToViewport` _returnvalue_2 0)
  (`WidgetBlueprintLibrary.SetInputMode_GameAndUIEx` _returnvalue _returnvalue_2 "DoNotLock" false)
  (set `PlayerController.bShowMouseCursor` true _returnvalue))

(fn `EndRound`
  (bind _returnvalue (`GameplayStatics.GetPlayerController` 0))
  (bind _endmenu (`self.EndMenu`))
  (`WidgetLayoutLibrary.RemoveAllWidgets`)
  (`UserWidget.AddToViewport` _endmenu 0)
  (`WidgetBlueprintLibrary.SetInputMode_UIOnlyEx` _returnvalue _endmenu)
  (set `PlayerController.bShowMouseCursor` true _returnvalue)
  (`/Game/GatchaAsset/Ui/EndMenu.update` _endmenu (`self.scores`)))

(fn `GetControllerIndex`
  (params (PlayerIndex :type Integer))
  (returns (ControllerIndex :type Integer))
  (switch `int` PlayerIndex
    (:`0`
      _)
    (:`1`
      _)
    (:`2`
      _)
    (:`3`
      _)
    (:`4`
      (return 1))
    (:`5`
      (return 1))
    (:`6`
      (return 2))
    (:`7`
      (return 2))
    (:`8`
      (return 3))
    (:`9`
      (return 3)))
  (return 0))

(fn `GetScoreWinner`
  (returns (Score :type Integer) (PlayerIndex :type Integer))
  (locals (`Highest score` :type Integer) (Index :type Integer))
  (for (_array_element _array_index) (`self.scores`)
    (if (>= _array_element (`local.Highest score`))
      (set `local.Highest score` _array_element)
      (set `local.Index` _array_index)))
  (return (`local.Highest score`) (`local.Index`)))

(fn `IncreaseSpeed`
  (set `self.LevelSpeed` (* (`KismetMathLibrary.Loge` (`self.IncrementValue`)) 1000.0))
  (set `self.IncrementValue` (+ (`self.IncrementValue`) 1.0)))

(fn `InstanciateControllers`
  (for _ (range 3)
    (`GameplayStatics.CreatePlayer` -1)))

(fn `killPlayer`
  (params (Player :type "/Game/GatchaAsset/Prog/Character/MyPlayer Object Reference"))
  (bind _returnvalue (`KismetArrayLibrary.Array_Length` (`self.Players`)))
  (`|ExecutionSequence`
    (:`then_1`
      (bind _outactors (`GameplayStatics.GetAllActorsOfClass` "/Game/GatchaAsset/Prog/Walls/BP_WallSpawner.BP_WallSpawner_C"))
      (`/Game/GatchaAsset/Prog/Walls/BP_WallSpawner.RemoveSpawnAt` (`|GetArrayItem` _outactors) Player))
    (:`then_2`
      (`self.SaveScore` Player)
      (`KismetArrayLibrary.Array_RemoveItem` (`self.Players`) Player)
      (`self.K2_DestroyActor` Player))
    (:`then_3`
      (if (== _returnvalue 0)
        (`self.EndRound`)
        (else
          (bind _outactors_2 (`GameplayStatics.GetAllActorsOfClass` "/Game/GatchaAsset/Prog/Audio/AudioManager.AudioManager_C"))
          (`/Game/GatchaAsset/Prog/Audio/AudioManager.Set SOUND` (`|GetArrayItem` _outactors_2) _returnvalue))))))

(fn `MoveAllPlayers`
  (params (DeltaTime :type "Float (double-precision)"))
  (bind _levelspeed (`self.LevelSpeed`))
  (bind _cameraactor (`self.CameraActor`))
  (`|ExecutionSequence`
    (:`then_0`
      (for _array_element (`self.Players`)
        (`self.K2_SetActorLocation` _array_element (+ (* (`self.GetActorForwardVector` _array_element) (* DeltaTime _levelspeed)) (`self.K2_GetActorLocation` _array_element)) false false)))
    (:`then_1`
      (`self.K2_SetActorLocation` _cameraactor (+ (* (`self.GetActorForwardVector` _cameraactor) (* DeltaTime _levelspeed)) (`self.K2_GetActorLocation` _cameraactor)) false false))))

(fn `removeHpPlayer`
  (params (PlayerIndex :type Integer))
  (bind _foundwidgets (`WidgetBlueprintLibrary.GetAllWidgetsOfClass` "/Game/GatchaAsset/Ui/GameUI.GameUI_C"))
  (`/Game/GatchaAsset/Ui/GameUI.RemoveHP` (`|GetArrayItem` _foundwidgets) PlayerIndex))

(fn `RemovePlayer`
  (bind _players (`self.Players`))
  (bind _returnvalue (- (`self.nbPlayers`) 1))
  (bind _asinput_controller (cast `/Game/GatchaAsset/Prog/Character/InputController` (`GameplayStatics.GetPlayerController` (`self.GetControllerIndex` (`self.nbPlayers`)))))
  (`/Game/GatchaAsset/Prog/Character/InputController.RemovePlayer` _asinput_controller)
  (`self.K2_DestroyActor` (`|GetArrayItem` _players _returnvalue))
  (`KismetArrayLibrary.Array_Remove` _players _returnvalue)
  (`/Engine/EditorBlueprintResources/StandardMacros.DecrementInt` (`self.nbPlayers`)))

(fn `ResetMovements`
  (`|ExecutionSequence`
    (:`then_0`
      (`self.trick`))
    (:`then_1`
      (set `self.IncrementValue` 2.0))
    (:`then_2`
      (`self.K2_SetActorLocation` (`self.CameraActor`) (-5320.0 -144.0 790.0) false false))))

(fn `resetScores`
  (bind _scores (`self.scores`))
  (for (_ _array_index) _scores
    (`KismetArrayLibrary.Array_Set` _scores _array_index)))

(fn `RespawnPlayers`
  (locals (tmp :type Integer))
  (bind _output_get (set `local.tmp` (`self.nbPlayers`)))
  (set `self.nbPlayers` 0)
  (for _ (range _output_get)
    (`self.AddPlayer`)))

(fn `restartLevel`
  (`|ExecutionSequence`
    (:`then_0`
      (`self.RespawnPlayers`))
    (:`then_1`
      (`self.resetScores`))
    (:`then_2`
      (`self.ResetMovements`))
    (:`then_3`
      (`self.CleanWalls`))
    (:`then_4`
      (`self.StartLevel`))))

(fn `SaveScore`
  (params (Player :type "/Game/GatchaAsset/Prog/Character/MyPlayer Object Reference"))
  (`KismetArrayLibrary.Array_Set` (`self.scores`) (`/Game/GatchaAsset/Prog/Character/MyPlayer.index` Player) (`/Game/GatchaAsset/Prog/Character/MyPlayer.score` Player)))

(fn `SetupPlayer`
  (params (PlayerIndex :type Integer))
  (returns (Index :type Integer) (Player :type "/Game/GatchaAsset/Prog/Character/MyPlayer Object Reference"))
  (bind _returnvalue (`|SpawnActorFromClass` "/Game/GatchaAsset/Prog/Character/MyPlayer.MyPlayer_C" (`self. GetRightSpawnTransform` null PlayerIndex) "AlwaysSpawn" "OverrideRootScale" null null))
  (`/Game/GatchaAsset/Prog/Character/MyPlayer.SetIndexPlayer` _returnvalue PlayerIndex)
  (`KismetArrayLibrary.Array_Add` (`self.Players`) _returnvalue)
  (return PlayerIndex _returnvalue))

(fn `StartLevel`
  (bind _returnvalue (`GameplayStatics.GetPlayerController` 0))
  (`|ExecutionSequence`
    (:`then_0`
      (bind _returnvalue_2 (`|CreateWidget` "/Game/GatchaAsset/Ui/GameUI.GameUI_C"))
      (`UserWidget.AddToViewport` _returnvalue_2 0)
      (`WidgetBlueprintLibrary.SetInputMode_GameOnly` _returnvalue)
      (set `PlayerController.bShowMouseCursor` false _returnvalue))
    (:`then_1`
      (`self.IncreaseSpeed`)
      (`KismetSystemLibrary.K2_SetTimer` self "IncreaseSpeed" 1.0 true))
    (:`then_2`
      (set `self.gameStarted` true)
      (`|SpawnActorFromClass` "/Game/GatchaAsset/Prog/Walls/BP_WallSpawner.BP_WallSpawner_C" (`KismetMathLibrary.MakeTransform` (0.0 0.0 0.0)) "Undefined" "OverrideRootScale" null null))))

(fn `UpdatePlayerScore`
  (params (playerIndex :type Integer) (Score :type Integer))
  (bind _foundwidgets (`WidgetBlueprintLibrary.GetAllWidgetsOfClass` "/Game/GatchaAsset/Ui/GameUI.GameUI_C"))
  (`/Game/GatchaAsset/Ui/GameUI.updateScore` (`|GetArrayItem` _foundwidgets) Score playerIndex))

(fn `UserConstructionScript`)