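; BP_WallSpawner spawns random walls along the X axis in each player's lane, at an accelerating rate.
; On BeginPlay it gathers MyPlayer actors, seeds the X position from the game mode's camera and starts spawning.
; Each SpawnWalls call places four evenly spaced walls from WallTypes at each player's Y, advances LastSpawnX and re-arms its timer with a shorter delay.
; RemoveSpawnAt drops a player from spawning.
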(event `self.ReceiveBeginPlay`
  (bind _returnvalue_x (`KismetMathLibrary.BreakVector` (`self.K2_GetActorLocation` (`self.Camera`))))
  (`|ExecutionSequence`
    (:`then_0`
      (bind _asbp_game_mode_gatcha (cast `/Game/GatchaAsset/Prog/GameModes/Bp_GameModeGatcha` (`GameplayStatics.GetGameMode`)))
      (set `self.Camera` (`/Game/GatchaAsset/Prog/GameModes/Bp_GameModeGatcha.CameraActor` _asbp_game_mode_gatcha)))
    (:`then_1`
      (bind _outactors (`GameplayStatics.GetAllActorsOfClass` "/Game/GatchaAsset/Prog/Character/MyPlayer.MyPlayer_C"))
      (set `self.Players` _outactors))
    (:`then_2`
      (`KismetSystemLibrary.K2_SetTimer` self "SpawnWalls" (`self.SpawnDelay`) true))
    (:`then_3`
      (set `self.LastSpawnX` _returnvalue_x)
      (`self.SpawnWalls`))))

(fn `RemoveSpawnAt`
  (params (Player :type "/Game/GatchaAsset/Prog/Character/MyPlayer Object Reference"))
  (`KismetArrayLibrary.Array_RemoveItem` (`self.Players`) Player))

(fn `SpawnWall`
  (params (PosX :type "Float (double-precision)") (PoxY :type "Float (double-precision)"))
  (bind _walltypes (`self.WallTypes`))
  (`|SpawnActorFromClass` (`|GetArrayItem` _walltypes (`KismetMathLibrary.RandomIntegerInRange` 0 (- (`KismetArrayLibrary.Array_Length` _walltypes) 1))) (`KismetMathLibrary.MakeTransform` (`KismetMathLibrary.MakeVector` PosX PoxY)) "Undefined" "OverrideRootScale" null null))

(fn `SpawnWalls`
  (bind _returnvalue (+ (`self.LastSpawnX`) (`self.SpawnDistance`)))
  (bind _returnvalue_2 (+ _returnvalue (`self.SpawnDistance`)))
  (bind _returnvalue_3 (+ _returnvalue_2 (`self.SpawnDistance`)))
  (bind _returnvalue_4 (+ _returnvalue_3 (`self.SpawnDistance`)))
  (for _array_element (`self.Players`)
    (bind (_returnvalue_x _returnvalue_y) (`KismetMathLibrary.BreakVector` (`self.K2_GetActorLocation` _array_element)))
    (`self.SpawnWall` _returnvalue _returnvalue_y)
    (`self.SpawnWall` _returnvalue_2 _returnvalue_y)
    (`self.SpawnWall` _returnvalue_3 _returnvalue_y)
    (`self.SpawnWall` _returnvalue_4 _returnvalue_y))
  (set `self.LastSpawnX` _returnvalue_4)
  (bind _output_get (set `self.SpawnDelay` (/ (`self.SpawnDelay`) 1.05)))
  (`KismetSystemLibrary.K2_SetTimer` null "SpawnWalls" _output_get))

(fn `UserConstructionScript`)