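; BP_Road is a road actor built from two instanced mesh components, Part1 and Part2, that can leapfrog to form a continuous road.
; The construction script extends each part by four instances, each spaced a fixed distance along X from the last.
; SwitchRoads alternately shifts one whole part along X by a five-section length plus a supplied offset, toggled by HasSwitched.
; RemoveRoadSection deletes Part1's first instance but is not called here.
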(event `self.ReceiveBeginPlay`)

(fn `AddRoadSection`
  (bind _part1 (`self.Part1`))
  (bind _outinstancetransform (`InstancedStaticMeshComponent.GetInstanceTransform` _part1 (`self.NbMap1`) false))
  (bind _returnvalue (`InstancedStaticMeshComponent.AddInstance` _part1 (`KismetMathLibrary.MakeTransform` (`KismetMathLibrary.MakeVector` (+ (.x (.location _outinstancetransform)) 25000.0) (.y (.location _outinstancetransform)) (.z (.location _outinstancetransform))) (.rotation _outinstancetransform) (.scale _outinstancetransform))))
  (set `self.NbMap1` _returnvalue))

(fn `AddRoadSection2`
  (bind _part2 (`self.Part2`))
  (bind _outinstancetransform (`InstancedStaticMeshComponent.GetInstanceTransform` _part2 (`self.NbMap2`) false))
  (bind _returnvalue (`InstancedStaticMeshComponent.AddInstance` _part2 (`KismetMathLibrary.MakeTransform` (`KismetMathLibrary.MakeVector` (+ (.x (.location _outinstancetransform)) 25000.0) (.y (.location _outinstancetransform)) (.z (.location _outinstancetransform))) (.rotation _outinstancetransform) (.scale _outinstancetransform))))
  (set `self.NbMap2` _returnvalue))

(fn `RemoveRoadSection`
  (`InstancedStaticMeshComponent.RemoveInstance` (`self.Part1`) 0))

(fn `SwitchRoads`
  (params (Offset :type "Float (double-precision)"))
  (bind _returnvalue (+ Offset 125000.0))
  (if (`self.HasSwitched?`)
    (`SceneComponent.K2_AddWorldOffset` (`self.Part2`) (`KismetMathLibrary.MakeVector` _returnvalue) false false)
    (set `self.HasSwitched?` false)
    (else
      (`SceneComponent.K2_AddWorldOffset` (`self.Part1`) (`KismetMathLibrary.MakeVector` _returnvalue) false false)
      (set `self.HasSwitched?` true))))

(fn `UserConstructionScript`
  (for _ (range 1 5)
    (`self.AddRoadSection`)
    (`self.AddRoadSection2`)))